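; BP_Attack is an actor Blueprint that rates an attack as strong or weak when play begins.
; CalculateAttack scales the STRStrength variable by a multiplier and adds a flat bonus.
; BeginPlay compares the result to a fixed threshold, then plays a matching 2D sound and prints the verdict on screen.
; It applies no damage, and its overlap and tick events are unused.
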(event EventBeginPlay
  (bind _attackvalue (CallFunction|CalculateAttack (Variables|Default|GetSTR%28Strength%29) 5 10))
  (if (>= _attackvalue 40)
    (Audio|PlaySound2D "/Game/StarterContent/Audio/Fire01_Cue.Fire01_Cue" 1.0 1.0 0.0 0 0)
    (Development|PrintString "STRONG ATTACK")
    (else
      (Audio|PlaySound2D "/Game/assets/Audio/BRUH.BRUH" 1.0 1.0 0.0 0 0)
      (Development|PrintString "WEAK ATTACK"))))

(event Collision|EventActorBeginOverlap
  (params (OtherActor :type Actor%20Object%20Reference)))

(event EventTick
  (params (DeltaSeconds :type Float%20%28single-precision%29)))

(fn ConstructionScript)

(fn CalculateAttack
  (params (StrengthValue :type Integer) (StrMult :type Integer) (StrAdd :type Integer))
  (return (+ (* StrengthValue StrMult) StrAdd)))